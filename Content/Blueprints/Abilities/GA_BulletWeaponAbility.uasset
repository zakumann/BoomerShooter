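; Base Gameplay Ability for bullet weapons, with an empty FireWeapon hook for subclasses to override.
; On activation it commits, listens for WeaponEventTag, fires, then ends when the remaining cooldown elapses, using it as the fire-rate delay.
; ApplyEffect sends hit targets to the attacker as that tagged event, and the listener applies WeaponEffect to them.
; Ending cleans up both async tasks and calls the empty Reset hook if the delay task is valid.
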(event `self.K2_ActivateAbility`
  ; Activation
  (`self.K2_CommitAbility`)
  (`self.WaitForEvent`)
  (`self.FireWeapon`)
  ; Ability Duration
  (bind _asynctaskproxy (`GameplayTask_WaitDelay.TaskWaitDelay` null (`self.GetCooldownTimeRemaining`))
    (:`then`
      (set `self.FireRateDelayTask` _asynctaskproxy))
    (:`OnFinish`
      (`self.K2_EndAbility`))))

(event `WaitForEvent`
  ; Wait for Gameplay Tag
  (bind (_asynctaskproxy _payload) (`AbilityTask_WaitGameplayEvent.WaitGameplayEvent` (`self.WeaponEventTag`) null)
    (:`then`
      (set `self.GameplayEventWaitTask` _asynctaskproxy))
    (:`EventReceived`
      (`self.BP_ApplyGameplayEffectToTarget` (`.TargetData` (break `GameplayEventData` _payload)) (`self.WeaponEffect`)))))

(event `FireWeapon`
  ; ToOverride
)

(event `self.K2_OnEndAbility`
  (params (bWasCancelled :type Boolean))
  (bind _gameplayeventwaittask (`self.GameplayEventWaitTask`))
  (bind _fireratedelaytask (`self.FireRateDelayTask`))
  ; End Ability Cleanup
  (`/Engine/EditorBlueprintResources/StandardMacros.IsValid` _gameplayeventwaittask
    (:`Is Valid`
      (`GameplayTask.EndTask` _gameplayeventwaittask))
    (:`Is Not Valid`
      _))
  (`/Engine/EditorBlueprintResources/StandardMacros.IsValid` _fireratedelaytask
    (:`Is Valid`
      (`GameplayTask.EndTask` _fireratedelaytask)
      (`self.Reset`))))

(fn `ApplyEffect`
  (params (AttackingActor :type "Actor Object Reference") (TargetActor :type "Actor Object Reference"))
  (`AbilitySystemBlueprintLibrary.SendGameplayEventToActor` AttackingActor (`self.WeaponEventTag`) (make `GameplayEventData` (struct) null TargetActor null null (struct) (struct) (struct) 0.0 (`AbilitySystemBlueprintLibrary.AbilityTargetDataFromActor` TargetActor))))

(fn `Reset`)