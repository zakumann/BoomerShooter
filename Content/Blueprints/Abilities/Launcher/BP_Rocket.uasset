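; Rocket projectile for the launcher ability, drawn as a Paper2D sprite that a looping timer yaws toward the player camera.
; When movement stops, it applies radial damage and a GAS rocket-damage effect to player characters directly hit or inside a separate explosion-radius overlap.
; Each character's own ability system component is both source and target of that effect.
; It then spawns an explosion actor aligned to the impact normal and destroys itself.
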(event `self.ReceiveBeginPlay`
  (`KismetSystemLibrary.K2_SetTimerDelegate` (delegate `DirectToPlayer`) 0.15 true)
  (`self.DirectToPlayer`))

(event `DirectToPlayer`
  (bind _papersprite (`self.PaperSprite`))
  (bind (_returnvalue_roll _returnvalue_pitch _returnvalue_yaw) (`KismetMathLibrary.BreakRotator` (`KismetMathLibrary.FindLookAtRotation` (`SceneComponent.K2_GetComponentLocation` _papersprite) (`PlayerCameraManager.GetCameraLocation` (`GameplayStatics.GetPlayerCameraManager` 0)))))
  (`SceneComponent.K2_SetWorldRotation` _papersprite (`KismetMathLibrary.MakeRotator` 0.0 0.0 (- _returnvalue_yaw 90.0)) false false))

(event `self.ProjectileMovement.OnProjectileStop`
  (params (ImpactResult :type "HitResult Structure (by ref)"))
  (bind _asbp_boomer_shooter_character (cast `/Game/Blueprints/BP_BoomerShooterCharacter` ImpactResult_HitActor)
    (:`then`
      (bind _returnvalue (`AbilitySystemBlueprintLibrary.GetAbilitySystemComponent` _asbp_boomer_shooter_character))
      (`AbilitySystemComponent.BP_ApplyGameplayEffectToTarget` _returnvalue "/Game/Blueprints/Abilities/Launcher/GE_PlayerRocketDamage.GE_PlayerRocketDamage_C" _returnvalue 0.0 (`AbilitySystemComponent.MakeEffectContext` _returnvalue)))
    (:`CastFailed`
      _))
  (`GameplayStatics.ApplyRadialDamage` :`BaseDamage` (`self.ExplosionDamage`) :`Origin` ImpactResult_ImpactPoint :`DamageRadius` (`self.Damage Radius`) :`DamageCauser` self :`InstigatedByController` null)
  (bind _outactors (`KismetSystemLibrary.SphereOverlapActors` ImpactResult_ImpactPoint (`self.ExplosionRadius`) (`self.Object Types`) null (`self.Actors to Ignore`)))
  (for _array_element _outactors
    (bind _asbp_boomer_shooter_character_2 (cast `/Game/Blueprints/BP_BoomerShooterCharacter` _array_element))
    (bind _returnvalue_2 (`AbilitySystemBlueprintLibrary.GetAbilitySystemComponent` _asbp_boomer_shooter_character_2))
    (`AbilitySystemComponent.BP_ApplyGameplayEffectToTarget` _returnvalue_2 "/Game/Blueprints/Abilities/Launcher/GE_PlayerRocketDamage.GE_PlayerRocketDamage_C" _returnvalue_2 0.0 (`AbilitySystemComponent.MakeEffectContext` _returnvalue_2)))
  (`|SpawnActorFromClass` "/Game/Blueprints/Abilities/Launcher/BP_RocketExplosion.BP_RocketExplosion_C" (`KismetMathLibrary.MakeTransform` ImpactResult_ImpactPoint (`KismetMathLibrary.Conv_VectorToRotator` ImpactResult_ImpactNormal)) "Undefined" "MultiplyWithRoot" null null)
  (`self.K2_DestroyActor`))

(fn `UserConstructionScript`)