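; Rocket explosion effect actor that displays a Paper2D flipbook sprite and then removes itself.
; On BeginPlay and on a short looping timer, it turns the flipbook in yaw only to face the player camera as a billboard.
; The same event starts a Delay of the flipbook's length, so the actor destroys itself one animation length after spawning.
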(event `self.ReceiveBeginPlay`
  (`KismetSystemLibrary.K2_SetTimerDelegate` (delegate `DirectToPlayer`) 0.15 true)
  (`self.DirectToPlayer`))

(event `DirectToPlayer`
  (bind _paperflipbook (`self.PaperFlipbook`))
  (bind (_returnvalue_roll _returnvalue_pitch _returnvalue_yaw) (`KismetMathLibrary.BreakRotator` (`KismetMathLibrary.FindLookAtRotation` (`SceneComponent.K2_GetComponentLocation` _paperflipbook) (`PlayerCameraManager.GetCameraLocation` (`GameplayStatics.GetPlayerCameraManager` 0)))))
  (`SceneComponent.K2_SetWorldRotation` _paperflipbook (`KismetMathLibrary.MakeRotator` 0.0 0.0 (- _returnvalue_yaw 90.0)) false false)
  (`KismetSystemLibrary.Delay` (`PaperFlipbookComponent.GetFlipbookLength` (`self.PaperFlipbook`)))
  (`self.K2_DestroyActor`))

(fn `UserConstructionScript`)