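; Gameplay ability for the pistol enemy's hitscan shot, run through its FireWeapon event.
; FireWeapon caches the owning BP_PistolEnemy, then line-traces on Visibility from its capsule along the forward vector out to WeaponRange, with persistent debug drawing.
; A player hit gets the ability's effect applied; any other hit places a bullet hole from the enemy's object pool, aligned to the surface normal.
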(event `self.FireWeapon`
  (`self.GetEnemy`)
  (bind _actor (`self.GetLineTrace`))
  (bind _asboomer_shooter_character (cast `BoomerShooterCharacter` _actor))
  (`self.ApplyEffect` (`self.PistolEnemy`) _asboomer_shooter_character))

(fn `GetEnemy`
  (bind _returnvalue_owneractor (break `GameplayAbilityActorInfo` (`self.GetActorInfo`)))
  (`/Engine/EditorBlueprintResources/StandardMacros.IsValid` (`self.PistolEnemy`)
    (:`Is Valid`
      _)
    (:`Is Not Valid`
      (bind _asbp_pistol_enemy (cast `/Game/Blueprints/Enemy/BP_PistolEnemy` _returnvalue_owneractor))
      (set `self.PistolEnemy` _asbp_pistol_enemy)))
  (return))

(fn `GetLineTrace`
  (returns (Actor :type "Actor Object Reference"))
  (bind _capsulecomponent (`Character.CapsuleComponent` (`self.PistolEnemy`)))
  (bind _returnvalue (`SceneComponent.K2_GetComponentLocation` _capsulecomponent))
  (bind (_outhit _returnvalue_2) (`KismetSystemLibrary.LineTraceSingle` :`Start` _returnvalue :`End` (+ _returnvalue (* (`KismetMathLibrary.GetForwardVector` (`SceneComponent.K2_GetComponentRotation` _capsulecomponent)) (`self.WeaponRange`))) :`TraceChannel` "TraceTypeQuery1" :`DrawDebugType` "Persistent"))
  (if _returnvalue_2
    (bind (_bblockinghit _binitialoverlap _time _distance _location _impactpoint _normal _impactnormal _physmat _hitactor) (`GameplayStatics.BreakHitResult` _outhit))
    (cast `/Game/Blueprints/Player/BP_FPSPlayer` _hitactor
      (:`then`
        (return _hitactor))
      (:`CastFailed`
        (bind _returnvalue_3 (`ObjectsPool.SpawnPooledObject` :`self` (`/Game/Blueprints/Enemy/BP_PistolEnemy.ObjectsPool-BulletHoles` (`self.PistolEnemy`)) :`SpawnLocation` _impactpoint))
        (`Actor.K2_SetActorLocation` _returnvalue_3 _impactpoint false false)
        (`Actor.K2_SetActorRotation` _returnvalue_3 (`KismetMathLibrary.Conv_VectorToRotator` _impactnormal) false)))))