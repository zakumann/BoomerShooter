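; Base character Blueprint for a boomer shooter, handling damage feedback and death detection through the Gameplay Ability System.
; TakeDamage receives cue data, prints health and armor readouts, and reports a damage event using the effect context's instigator and the cue's location.
; HealthCheck then tests an ability system attribute for zero or below, triggering KillCharacter, which is an empty event here, as is BeginPlay.
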(event `self.ReceiveBeginPlay`)

(event `TakeDamage`
  (params (CueData :type "GameplayCueParameters Structure"))
  (bind (_normalizedmagnitude _rawmagnitude _effectcontext _matchedtagname _originaltag _aggregatedsourcetags _aggregatedtargettags _location) (`AbilitySystemBlueprintLibrary.BreakGameplayCueParameters` CueData))
  (bind _abilitysystemcomponent (`self.AbilitySystemComponent`))
  (`KismetSystemLibrary.PrintString` (`KismetStringLibrary.Concat_StrStr` "Health: " (`KismetStringLibrary.Conv_DoubleToString` (`.ReturnValue` (`AbilitySystemBlueprintLibrary.GetFloatAttributeFromAbilitySystemComponent` _abilitysystemcomponent (struct :`AttributeName` "Health" :`Attribute` "/Script/BoomerShooter.BoomerShooterAttributeSet:Health" :`AttributeOwner` "/Script/CoreUObject.Class'/Script/BoomerShooter.BoomerShooterAttributeSet'")))) ", Armor: " (`KismetStringLibrary.Conv_DoubleToString` (`.ReturnValue` (`AbilitySystemBlueprintLibrary.GetFloatAttributeFromAbilitySystemComponent` _abilitysystemcomponent (struct :`AttributeName` "Armor" :`Attribute` "/Script/BoomerShooter.BoomerShooterAttributeSet:Armor" :`AttributeOwner` "/Script/CoreUObject.Class'/Script/BoomerShooter.BoomerShooterAttributeSet'"))))) true true (struct :`G` 0.66 :`B` 1.0 :`A` 1.0) 60.0)
  (`AISense_Damage.ReportDamageEvent` self (`AbilitySystemBlueprintLibrary.EffectContextGetInstigatorActor` _effectcontext) 0.0 _location)
  (if (`self.HealthCheck`)
    (`self.KillCharacter`)))

(event `KillCharacter`)

(fn `HealthCheck`
  (returns (bIsDead :type Boolean))
  (return (<= (`.ReturnValue` (`AbilitySystemBlueprintLibrary.GetFloatAttributeFromAbilitySystemComponent` (`self.AbilitySystemComponent`) (struct :`AttributeName` "Health" :`Attribute` "/Script/BoomerShooter.BoomerShooterAttributeSet:Health" :`AttributeOwner` "/Script/CoreUObject.Class'/Script/BoomerShooter.BoomerShooterAttributeSet'"))) 0.0)))

(fn `UserConstructionScript`)