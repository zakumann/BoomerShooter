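; BP_Enemy is an enemy drawn as a billboarded Paper2D flipbook that shows directional sprites based on the player's viewing angle, Doom-style.
; A looping timer, started at BeginPlay, yaws the sprite toward the camera, then computes the flat angle between the actor's forward vector and the player.
; A right-vector dot product picks the visible side, and angle thresholds map the result to one of eight directional flipbooks.
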(event `self.ReceiveBeginPlay`
  (`KismetSystemLibrary.K2_SetTimerDelegate` (delegate `DirectToPlayer`) 0.15 true)
  (`self.DirectToPlayer`))

(event `DirectToPlayer`
  (`self.SpriteFacePlayer`
    (:`Out`
      (`self.GetEnemyAngle`
        (:`Out`
          (`self.CalculateFlipbook`))))))

(fn `UserConstructionScript`)