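; Pistol-wielding enemy Blueprint that supplies a ranged attack through the Gameplay Ability System.
; The RangedAttack event activates abilities by gameplay tag on the AbilitySystemComponent, then briefly reveals a PointLight, apparently as a muzzle flash.
; A short Delay hides the light again; the flash plays regardless of whether activation succeeds.
; BeginPlay, overlap and Tick are disabled stubs, and the construction script only calls its parent.
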(event `self.RangedAttack`
  (`AbilitySystemComponent.TryActivateAbilitiesByTag` (`self.AbilitySystemComponent`) (`self.Gameplay Tag Container`) false)
  (`SceneComponent.SetHiddenInGame` (`self.PointLight`) false false)
  (`KismetSystemLibrary.Delay` 0.2)
  (`SceneComponent.SetHiddenInGame` (`self.PointLight`) true false))

(fn `UserConstructionScript`
  (`parent.UserConstructionScript`))