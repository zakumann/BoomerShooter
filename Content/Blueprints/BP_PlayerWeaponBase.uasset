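; Base Blueprint for player weapons, displayed as a 2D flipbook isolated by a SceneCapture2D show-only component.
; InitializeWeapon clears and hides the flipbook, and DrawWeapon uses a timeline to raise it into view, saving its position as the rest location.
; WeaponBob nudges the flipbook along Y with a timeline while moving, then stops and interpolates back to that saved location when idle.
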(event `self.ReceiveBeginPlay`
  (`SceneCaptureComponent.ShowOnlyComponent` (`self.SceneCaptureComponent2D`) (`self.WeaponFlipbook`)))

(event `/Game/Interfaces/INT_PlayerWeapon.InitializeWeapon`
  (bind _weaponflipbook (`self.WeaponFlipbook`))
  (`PaperFlipbookComponent.SetFlipbook` _weaponflipbook null)
  (`SceneComponent.SetHiddenInGame` _weaponflipbook true false))

(event `WeaponBob`
  (params (bIsMoving :type Boolean) (DeltaTime :type "Float (double-precision)"))
  (bind _weaponflipbook (`self.WeaponFlipbook`))
  (bind (_relativelocation_x _relativelocation_y _relativelocation_z) (`KismetMathLibrary.BreakVector` (`SceneComponent.RelativeLocation` _weaponflipbook)))
  (if bIsMoving
    (bind (_direction _weaponbobtracck) (`Timeline|T_WeaponBob` :!label _label)
      (:`Update`
        (`SceneComponent.K2_SetRelativeLocation` _weaponflipbook (`KismetMathLibrary.MakeVector` _relativelocation_x (`KismetMathLibrary.Lerp` (+ _relativelocation_y 0.2) (- _relativelocation_y 0.2) _weaponbobtracck) _relativelocation_z) false false)))
    (else
      (`|ExecutionSequence`
        (:`then_0`
          (goto _label :!via `Stop`))
        (:`then_1`
          (`SceneComponent.K2_SetRelativeLocation` (`self.WeaponFlipbook`) (`KismetMathLibrary.VInterpTo` (`SceneComponent.RelativeLocation` (`self.WeaponFlipbook`)) (`self.FlipbookLocation`) DeltaTime 50.0) false false))))))

(event `DrawWeapon`
  ; WeaponDraw
  (bind (_direction _alpha) (`Timeline|T_DrawTimeline` :!via `PlayFromStart`)
    (:`Update`
      (`SceneComponent.K2_SetRelativeLocation` (`self.WeaponFlipbook`) (`KismetMathLibrary.VLerp` (0.0 100.0 -120.0) (0.0 100.0 -50.0) _alpha) false false)
      ; WeaponLocation
      (set `self.FlipbookLocation` (`SceneComponent.RelativeLocation` (`self.WeaponFlipbook`))))))

(fn `UserConstructionScript`)