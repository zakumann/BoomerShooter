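; BP_Launcher is the rocket launcher weapon for the FPS player, drawn as an animated Paper2D flipbook.
; InitializeWeapon shows the idle flipbook and caches the BP_FPSPlayer pawn.
; ShootLauncher triggers a brief point-light muzzle flash, refreshes the player's UI and spawns a BP_Rocket at the spawn point.
; It then plays the fire flipbook for its length before returning to idle.
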(event `self.InitializeWeapon`
  ; Equip Weapon
  (`PaperFlipbookComponent.SetFlipbook` (`self.WeaponFlipbook`) (`self.IdleLauncher`))
  (`SceneComponent.SetHiddenInGame` (`self.WeaponFlipbook`) false false)
  (bind _asbp_fpsplayer (cast `/Game/Blueprints/Player/BP_FPSPlayer` (`GameplayStatics.GetPlayerPawn` 0)))
  (set `self.Player` _asbp_fpsplayer))

(event `ShootLauncher`
  (bind _weaponflipbook (`self.WeaponFlipbook`))
  ; Launcher Fire Animation
  (`self.LightFlash`)
  (`/Game/Blueprints/Player/BP_FPSPlayer.UpdateUI` (`self.Player`))
  (`|SpawnActorFromClass` "/Game/Blueprints/Abilities/Launcher/BP_Rocket.BP_Rocket_C" (`SceneComponent.K2_GetComponentToWorld` (`self.RocketSpawnPoint`)) "Undefined" "MultiplyWithRoot" null null)
  (`PaperFlipbookComponent.SetFlipbook` _weaponflipbook (`self.FireLauncher`))
  (`KismetSystemLibrary.Delay` (`PaperFlipbookComponent.GetFlipbookLength` _weaponflipbook))
  (`PaperFlipbookComponent.SetFlipbook` (`self.WeaponFlipbook`) (`self.IdleLauncher`)))

(event `LightFlash`
  (bind _pointlight (`self.PointLight`))
  ; Light Flash
  (`SceneComponent.SetHiddenInGame` _pointlight false false)
  (`KismetSystemLibrary.Delay` 0.15)
  (`SceneComponent.SetHiddenInGame` _pointlight true false))

(fn `UserConstructionScript`
  (`parent.UserConstructionScript`))