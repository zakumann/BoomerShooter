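; BP_Pistol is a pistol weapon Blueprint that handles the visuals for equipping and firing, using Paper2D flipbook animation.
; InitializeWeapon shows the weapon flipbook in its idle animation.
; ShootPistol triggers a brief point-light muzzle flash and plays the fire flipbook, waiting for that flipbook's length before returning to idle.
; It contains no damage, trace or ammo logic, and its construction script only calls the parent's.
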(event `/Game/Blueprints/Interfaces/INT_PlayerWeapon.InitializeWeapon`
  ; Equip Weapon
  (`PaperFlipbookComponent.SetFlipbook` (`self.WeaponFlipbook`) (`self.IdlePistol`))
  (`SceneComponent.SetHiddenInGame` (`self.WeaponFlipbook`) false false))

(event `ShootPistol`
  (bind _weaponflipbook (`self.WeaponFlipbook`))
  ; Pistol Fire Animation
  (`self.LightFlash`)
  (`PaperFlipbookComponent.SetFlipbook` _weaponflipbook (`self.FirePistol`))
  (`KismetSystemLibrary.Delay` (`PaperFlipbookComponent.GetFlipbookLength` _weaponflipbook))
  (`PaperFlipbookComponent.SetFlipbook` (`self.WeaponFlipbook`) (`self.IdlePistol`)))

(event `LightFlash`
  (bind _pointlight (`self.PointLight`))
  ; Light Flash
  (`SceneComponent.SetHiddenInGame` _pointlight false false)
  (`KismetSystemLibrary.Delay` 0.15)
  (`SceneComponent.SetHiddenInGame` _pointlight true false))

(fn `UserConstructionScript`
  (`parent.UserConstructionScript`))