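; BP_Shotgun is the player's shotgun weapon, displayed as a flipbook sprite with a muzzle-flash light.
; Initialization shows the idle flipbook and caches the BP_FPSPlayer pawn.
; Firing briefly flashes the point light, updates the player's UI, and plays the fire flipbook, returning to idle after a delay equal to that flipbook's length.
; A sound playback node is present but never runs.
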(event `self.InitializeWeapon`
  ; Equip Weapon
  (`PaperFlipbookComponent.SetFlipbook` (`self.WeaponFlipbook`) (`self.IdleShotgun`))
  (`SceneComponent.SetHiddenInGame` (`self.WeaponFlipbook`) false false)
  (bind _asbp_fpsplayer (cast `/Game/Blueprints/Player/BP_FPSPlayer` (`GameplayStatics.GetPlayerPawn` 0)))
  (set `self.Player` _asbp_fpsplayer))

(event `ShootShotgun`
  (bind _weaponflipbook (`self.WeaponFlipbook`))
  ; Shotgun Fire Animation
  (`self.LightFlash`)
  (`/Game/Blueprints/Player/BP_FPSPlayer.UpdateUI` (`self.Player`))
  (`PaperFlipbookComponent.SetFlipbook` _weaponflipbook (`self.FireShotgun`))
  (`KismetSystemLibrary.Delay` (`PaperFlipbookComponent.GetFlipbookLength` _weaponflipbook))
  (`PaperFlipbookComponent.SetFlipbook` (`self.WeaponFlipbook`) (`self.IdleShotgun`)))

(event `LightFlash`
  (bind _pointlight (`self.PointLight`))
  ; Light Flash
  (`SceneComponent.SetHiddenInGame` _pointlight false false)
  (`KismetSystemLibrary.Delay` 0.15)
  (`SceneComponent.SetHiddenInGame` _pointlight true false))

(fn `UserConstructionScript`
  (`parent.UserConstructionScript`))