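; BP_WeaponPickup is a weapon pickup that gives its configured weapon to the player on overlap.
; A looping timer started at BeginPlay, used instead of Tick, periodically turns the Weapon component on yaw only to face the player camera, with an offset.
; When a BP_FPSPlayer overlaps it, the pickup passes WeapontoAcquire to EquipWeapon and destroys itself.
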(event `self.ReceiveBeginPlay`
  (`KismetSystemLibrary.K2_SetTimerDelegate` (delegate `DirectToPlayer`) 0.15 true)
  (`self.DirecttoPlayer`))

(event `DirectToPlayer`
  (bind _weapon (`self.Weapon`))
  (bind (_returnvalue_roll _returnvalue_pitch _returnvalue_yaw) (`KismetMathLibrary.BreakRotator` (`KismetMathLibrary.FindLookAtRotation` (`SceneComponent.K2_GetComponentLocation` _weapon) (`PlayerCameraManager.GetCameraLocation` (`GameplayStatics.GetPlayerCameraManager` 0)))))
  (`SceneComponent.K2_SetWorldRotation` _weapon (`KismetMathLibrary.MakeRotator` 0.0 0.0 (- _returnvalue_yaw 90.0)) false false))

(event `self.ReceiveActorBeginOverlap`
  (params (OtherActor :type "Actor Object Reference"))
  (bind _asbp_fpsplayer (cast `/Game/Blueprints/BP_FPSPlayer` OtherActor))
  (`/Game/Blueprints/BP_FPSPlayer.EquipWeapon` _asbp_fpsplayer (`self.WeapontoAcquire`))
  (`self.K2_DestroyActor`))

(fn `UserConstructionScript`)