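; A health or armor pickup, in small or large size, shown as a flipbook item.
; The construction script picks the flipbook, scale and gameplay tag from pickup type and size.
; Two check functions read a float attribute from a given Ability System and add or remove a Player Full tag in the pickup's tag at exactly 100.
; The event graph is empty, and nothing here calls those checks.
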(fn `FullArmorCheck`
  (params (AbilitySystem :type "AbilitySystemComponent Object Reference"))
  (bind _pickuptag (`self.PickupTag`))
  (if (== (`.ReturnValue` (`AbilitySystemBlueprintLibrary.GetFloatAttributeFromAbilitySystemComponent` AbilitySystem (struct :`AttributeName` "Armor" :`Attribute` "/Script/BoomerShooter.BoomerShooterAttributeSet:Armor" :`AttributeOwner` "/Script/CoreUObject.Class'/Script/BoomerShooter.BoomerShooterAttributeSet'"))) 100.0)
    (`BlueprintGameplayTagLibrary.AddGameplayTag` _pickuptag (struct :`TagName` "Player.Armor.Full"))
    (else
      (`BlueprintGameplayTagLibrary.RemoveGameplayTag` _pickuptag (struct :`TagName` "Player.Armor.Full")))))

(fn `FullHealthCheck`
  (params (AbilitySystem :type "AbilitySystemComponent Object Reference"))
  (bind _pickuptag (`self.PickupTag`))
  (if (== (`.ReturnValue` (`AbilitySystemBlueprintLibrary.GetFloatAttributeFromAbilitySystemComponent` AbilitySystem (struct :`AttributeName` "Health" :`Attribute` "/Script/BoomerShooter.BoomerShooterAttributeSet:Health" :`AttributeOwner` "/Script/CoreUObject.Class'/Script/BoomerShooter.BoomerShooterAttributeSet'"))) 100.0)
    (`BlueprintGameplayTagLibrary.AddGameplayTag` _pickuptag (struct :`TagName` "Player.Health.Full"))
    (else
      (`BlueprintGameplayTagLibrary.RemoveGameplayTag` _pickuptag (struct :`TagName` "Player.Health.Full")))))

(fn `SetStatPickupFlipbook`
  (bind _item (`self.Item`))
  (bind _item_2 (`self.Item`))
  (switch `/Game/Blueprints/ENUMs/ENUM_PickupType` (`self.PickupType`)
    (:`NewEnumerator0`
      (`PaperFlipbookComponent.SetFlipbook` _item "/Game/Flipbooks/Pickups/FB_ArmorPickup.FB_ArmorPickup")
      (switch `/Game/Blueprints/ENUMs/ENUM_PickupSize` (`self.PickupSize`)
        (:`NewEnumerator0`
          (`SceneComponent.SetRelativeScale3D` _item_2 (1.0 1.0 1.0))
          (set `self.PickupTag` (struct :`GameplayTags` (struct :`(TagName` "Pickup.Armor.Small")))))
        (:`NewEnumerator1`
          (`SceneComponent.SetRelativeScale3D` _item_2 (2.0 2.0 2.0))
          (set `self.PickupTag` (struct :`GameplayTags` (struct :`(TagName` "Pickup.Armor.Large")))))))
    (:`NewEnumerator1`
      (`PaperFlipbookComponent.SetFlipbook` _item "/Game/Flipbooks/Pickups/FB_HealthPickup.FB_HealthPickup")
      (switch `/Game/Blueprints/ENUMs/ENUM_PickupSize` (`self.PickupSize`)
        (:`NewEnumerator0`
          (`SceneComponent.SetRelativeScale3D` _item_2 (1.0 1.0 1.0))
          (set `self.PickupTag` (struct :`GameplayTags` (struct :`(TagName` "Pickup.Health.Small")))))
        (:`NewEnumerator1`
          (`SceneComponent.SetRelativeScale3D` _item_2 (2.0 2.0 2.0))
          (set `self.PickupTag` (struct :`GameplayTags` (struct :`(TagName` "Pickup.Health.Large")))))))))

(fn `UserConstructionScript`
  (`parent.UserConstructionScript`)
  (`self.SetStatPickupFlipbook`))