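; Weapon pickup actor that grants a configurable weapon to the player who touches it.
; The construction script sets the Item flipbook sprite from the WeapontoAcquire enum, so each placed pickup previews its weapon in the editor.
; On overlap with BP_FPSPlayer, it calls PickupWeapon with that weapon type and destroys itself; other actors are ignored.
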(event `self.ReceiveActorBeginOverlap`
  (params (OtherActor :type "Actor Object Reference"))
  (bind _asbp_fpsplayer (cast `/Game/Blueprints/Player/BP_FPSPlayer` OtherActor))
  (`/Game/Blueprints/Player/BP_FPSPlayer.PickupWeapon` _asbp_fpsplayer (`self.WeapontoAcquire`))
  (`self.K2_DestroyActor`))

(fn `UserConstructionScript`
  (bind _item (`self.Item`))
  (switch `/Game/Blueprints/ENUMs/ENUM_WeaponList` (`self.WeapontoAcquire`)
    (:`NewEnumerator0`
      (`PaperFlipbookComponent.SetFlipbook` _item null))
    (:`NewEnumerator1`
      (`PaperFlipbookComponent.SetFlipbook` _item "/Game/Flipbooks/Pickups/FB_Pistol.FB_Pistol"))
    (:`NewEnumerator2`
      (`PaperFlipbookComponent.SetFlipbook` _item "/Game/Flipbooks/Pickups/FB_LauncherPickup.FB_LauncherPickup"))
    (:`NewEnumerator3`
      (`PaperFlipbookComponent.SetFlipbook` _item "/Game/Flipbooks/Pickups/FB_Shotgun.FB_Shotgun"))
    (:`NewEnumerator4`
      (`PaperFlipbookComponent.SetFlipbook` _item "/Game/Flipbooks/Pickups/FB_Chaingun.FB_Chaingun"))))